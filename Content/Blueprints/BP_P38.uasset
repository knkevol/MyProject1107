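; BP_P38 is a player-controlled P-38 aircraft that can pitch, roll and fire rockets.
; Pitch and Roll axis inputs add local rotation, scaled by delta seconds and a fixed rate for frame-rate-independent turning.
; Pressing Fire spawns a BP_Rocket at the Arrow component's world transform, with the aircraft as owner and instigator.
; The graph contains no forward movement logic.
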(event Input|ActionEvents|InputActionFire
  (params (Key :type Key%20Structure :default "None"))
  (bind _self self)
  (:Pressed
    (Game|SpawnActorfromClass "/Game/Blueprints/BP_Rocket.BP_Rocket_C" (Transformation|GetWorldTransform (Variables|Default|GetArrow)) "Undefined" "MultiplyWithRoot" _self _self)))

(event Input|AxisEvents|InputAxisPitch
  (params (AxisValue :type Float%20%28single-precision%29))
  (Transformation|AddActorLocalRotation (Math|Rotator|MakeRotator 0.0 (* AxisValue (Utilities|Time|GetWorldDeltaSeconds) 45.0) 0.0) false false))

(event Input|AxisEvents|InputAxisRoll
  (params (AxisValue :type Float%20%28single-precision%29))
  (Transformation|AddActorLocalRotation (Math|Rotator|MakeRotator (* AxisValue (Utilities|Time|GetWorldDeltaSeconds) 45.0) 0.0 0.0) false false))

(fn ConstructionScript)