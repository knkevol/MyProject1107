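; BP_Rocket is a short-lived projectile actor that destroys Target-tagged actors on overlap.
; It sets a lifespan on BeginPlay so it expires after a few seconds.
; On hitting a target it plays a sound and particle effect, calls Rule on the BP_GM game mode, then destroys itself.
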(event Collision|EventActorBeginOverlap
  (params (OtherActor :type Actor%20Object%20Reference))
  (if (Actor|ActorHasTag OtherActor "Target")
    (Actor|DestroyActor OtherActor)
    (Audio|SpawnSoundatLocation "/Engine/EngineSounds/1kSineTonePing.1kSineTonePing" (Transformation|GetActorLocation) "0, 0, 0" 1.0 1.0 0.0 0 0)
    (Effects|SpawnEmitteratLocation "/Engine/Tutorial/SubEditors/TutorialAssets/TutorialParticleSystem.TutorialParticleSystem" (Transformation|GetActorLocation))
    (bind _asbp_gm (Utilities|Casting|CastToBP_GM (Game|GetGameMode)))
    (Default|Rule _asbp_gm)
    (Actor|DestroyActor)))

(event EventBeginPlay
  (Actor|SetLifeSpan 3.0))

(fn ConstructionScript)